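; BP_Crystal is a collectible crystal actor that flies into the player and disappears when the player overlaps it.
; On overlap it stores its starting location, scale and point light intensity, then plays a collection timeline.
; Timeline curves lerp it toward the player pawn's current position each update, shrink it to zero and fade its light.
; The actor destroys itself when the timeline finishes.
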(event `self.ReceiveActorBeginOverlap`
  (params (OtherActor :type "Actor Object Reference"))
  (`/Game/Blueprints/Libraries/ML_Actor_Macro_Library.IsPlayer` OtherActor
    (:`IsPlayer`
      (`self.Store Starting Values`)
      (bind (_direction _collection_progress _scale_progress _light_adjust) (`Timeline|Collection Timeline`)
        (:`Update`
          (`self.Move to Player Pawn` _collection_progress)
          (`self.Scale Crystal` _scale_progress)
          (`self.Light Adjust` _light_adjust))
        (:`Finished`
          (`self.K2_DestroyActor`))))))

(fn `Light Adjust`
  (params (Alpha :type "Float (double-precision)"))
  (`LightComponent.SetIntensity` (`self.PointLight`) (`KismetMathLibrary.Lerp` (`self.Starting Intensity`) 0.0 Alpha)))

(fn `Move to Player Pawn`
  (params (Alpha :type "Float (double-precision)"))
  (`self.K2_SetActorLocation` (`KismetMathLibrary.VLerp` (`self.Start Location`) (`self.K2_GetActorLocation` (`GameplayStatics.GetPlayerPawn` 0)) Alpha)))

(fn `Scale Crystal`
  (params (Alpha :type "Float (double-precision)"))
  (`self.SetActorScale3D` (`KismetMathLibrary.VLerp` (`self.Starting Scale`) (0.0 0.0 0.0) Alpha)))

(fn `Store Starting Values`
  (set `self.Start Location` (`self.K2_GetActorLocation`))
  (set `self.Starting Scale` (`self.GetActorScale3D`))
  (set `self.Starting Intensity` (`LightComponentBase.Intensity` (`self.PointLight`))))

(fn `UserConstructionScript`)