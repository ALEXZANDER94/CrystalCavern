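; BP_Cannon is a cannon actor that fires automatically and repeatedly from BeginPlay.
; After a CannonFireRate delay it spawns a BP_Projectile at ProjectileSpawnPoint's location and rotation, scaled by ProjectileScale.
; The CannonFireAnimation timeline then drives CannonHead's relative location to animate the barrel, and its Cannon Fired event track loops back to the delay for the next shot.
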(event `self.ReceiveBeginPlay`
  (`KismetSystemLibrary.Delay` (`self.CannonFire_Rate`) :!label _label)
  (`self.Fire Cannon` (`self.Projectile_Scale`))
  (bind (_direction _cannon_barrel_location) (`Timeline|Cannon Fire Animation` :!via `PlayFromStart`)
    (:`Update`
      (`self.Move_Cannon_Barrel` _cannon_barrel_location))
    (:`Cannon_Fired`
      (goto _label))))

(fn `Fire Cannon`
  (params (InFloat :type "Float (double-precision)"))
  (bind _projectile_spawn_point (`self.Projectile_Spawn_Point`))
  (`|SpawnActorFromClass` "/Game/Blueprints/Actors/Projectiles/BP_Projectile.BP_Projectile_C" (`KismetMathLibrary.MakeTransform` (`SceneComponent.K2_GetComponentLocation` _projectile_spawn_point) (`SceneComponent.K2_GetComponentRotation` _projectile_spawn_point) (`KismetMathLibrary.Conv_DoubleToVector` InFloat)) "Undefined" "OverrideRootScale" null null))

(fn `Move_Cannon_Barrel`
  (params (NewLocation_Y :type "Float (double-precision)"))
  (`SceneComponent.K2_SetRelativeLocation` (`self.CannonHead`) (`KismetMathLibrary.MakeVector` 0.0 NewLocation_Y) false false))

(fn `UserConstructionScript`)